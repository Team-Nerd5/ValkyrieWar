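; Gameplay Ability for the Valkyrie character's four-step bow attack combo.
; On activation it calls Attack on the avatar character, then uses its ComboCount to choose one of four bow montages.
; Every montage task outcome, including Blended In, ends the ability, so it does not wait for the animation to finish.
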(event Ability|EventOnEndAbility
  (params (bWasCancelled :type Boolean)))

(event Ability|EventActivateAbility
  (Development|PrintString "스킬발동 켜짐")
  (bind _returnvalue (Ability|GetAvatarActorfromActorInfo))
  (bind _asvalkyrie_character (Utilities|Casting|CastToValkyrieCharacter _returnvalue))
  (Class|ValkyrieCharacter|Attack _asvalkyrie_character)
  (switch int (Variables|/Script/ValkyrieWar.ValkyrieCharacter|GetComboCount _asvalkyrie_character)
    (:0
      (|PlayMontageandWaitProxy "None" "/Game/ExternalContents/Valkyries/ArcherElves/Animation/Montage/Attack/Bow_Combo1.Bow_Combo1" 1.0 "None" true 1.0 0.0 false
        (:OnCompleted
          _)
        (:OnBlendedIn
          _)
        (:OnBlendOut
          _)
        (:OnInterrupted
          _)
        (:OnCancelled
          _)))
    (:1
      (|PlayMontageandWaitProxy "None" "/Game/ExternalContents/Valkyries/ArcherElves/Animation/Montage/Attack/Bow_Combo2.Bow_Combo2" 1.0 "None" true 1.0 0.0 false
        (:OnCompleted
          _)
        (:OnBlendedIn
          _)
        (:OnBlendOut
          _)
        (:OnInterrupted
          _)
        (:OnCancelled
          _)))
    (:2
      (|PlayMontageandWaitProxy "None" "/Game/ExternalContents/Valkyries/ArcherElves/Animation/Montage/Attack/Bow_Combo3.Bow_Combo3" 1.0 "None" true 1.0 0.0 false
        (:OnCompleted
          _)
        (:OnBlendedIn
          _)
        (:OnBlendOut
          _)
        (:OnInterrupted
          _)
        (:OnCancelled
          _)))
    (:3
      (|PlayMontageandWaitProxy "None" "/Game/ExternalContents/Valkyries/ArcherElves/Animation/Montage/Attack/Bow_Combo4.Bow_Combo4" 1.0 "None" true 1.0 0.0 false
        (:OnCompleted
          _)
        (:OnBlendedIn
          _)
        (:OnBlendOut
          _)
        (:OnInterrupted
          _)
        (:OnCancelled
          _))))
  (Ability|EndAbility))