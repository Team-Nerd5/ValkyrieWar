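; Actor Blueprint that plays a three-stage Niagara effect sequence (spawn, loop, death) on repeat, likely for showcasing VFX.
; On BeginPlay it activates the spawn and loop components together, then a timer ends the loop after LoopTime.
; Ending deactivates the loop and fires the death effect, and a second timer restarts the sequence after DelayBetweenLoop.
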(event Custom|EndLoop
  (Components|Activation|Deactivate (Variables|Default|GetNiagaraLoop))
  (Components|Activation|Activate (Variables|Default|GetNiagaraDeath) true)
  (Utilities|Time|SetTimerbyEvent (delegate Custom|PlayVFX) (Variables|Default|GetDelayBetweenLoop)))

(event Custom|PlayVFX
  (Components|Activation|Activate (Variables|Default|GetNiagaraSpawn) true)
  (Utilities|Time|SetTimerbyEvent (delegate Custom|EndLoop) (Variables|Default|GetLoopTime)))

(event EventBeginPlay
  (CallFunction|PlayVFX))

(event Collision|EventActorBeginOverlap
  (params (OtherActor :type Actor%20Object%20Reference)))

(event EventTick
  (params (DeltaSeconds :type Float%20%28single-precision%29)))

(fn ConstructionScript)