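; Playable Valkyrie hooded archer elf pawn, moved by an on-screen joystick widget.
; BeginPlay creates WBP_MoveUI, stores it as the joystick reference and adds it to the viewport.
; Tick feeds the widget's JoyStickAxis into movement input along fixed world forward and right axes, with Y inverted, so movement ignores camera and actor rotation.
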(event EventBeginPlay
  (bind _returnvalue (UserInterface|CreateWidget "/Game/GameSystem/UI/WBP_MoveUI.WBP_MoveUI_C"))
  (bind _output_get (Variables|Default|SetRef_JoyStick _returnvalue))
  (UserInterface|Viewport|AddtoViewport _output_get 0))

(event Collision|EventActorBeginOverlap
  (params (OtherActor :type Actor%20Object%20Reference)))

(event EventTick
  (params (DeltaSeconds :type Float%20%28single-precision%29))
  (bind _ref_joystick (Variables|Default|GetRef_JoyStick))
  (bind _joystickaxis (Variables|/Game/GameSystem/UI/WBP_MoveUI.WBP_MoveUI_C|GetJoyStickAxis _ref_joystick))
  (Pawn|Input|AddMovementInput (Math|Vector|GetForwardVector "0, 0, 0") (* (.y _joystickaxis) -1.0) false)
  (Pawn|Input|AddMovementInput (Math|Vector|GetRightVector "0, 0, 0") (.x _joystickaxis) false))

(fn ConstructionScript)