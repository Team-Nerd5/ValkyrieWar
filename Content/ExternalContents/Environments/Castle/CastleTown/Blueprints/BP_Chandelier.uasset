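; Castle town chandelier prop that hangs an iron chandelier mesh from a procedurally built chain of adjustable length.
; The construction script lowers the chandelier by ChainLength and moves the chain spline's second point to match.
; It then places Z-forward spline mesh links along the spline, spaced by the link mesh's bounding-box height, with tangents clamped to link length.
; The event graph holds no active logic.
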(event EventBeginPlay)

(event Collision|EventActorBeginOverlap
  (params (OtherActor :type Actor%20Object%20Reference)))

(event EventTick
  (params (DeltaSeconds :type Float%20%28single-precision%29)))

(fn ConstructionScript
  (bind _chain_length (Variables|Default|GetChain%20Length))
  (bind _chainlink (Variables|Default|GetChainLink))
  (bind _chainspline (Variables|Default|GetChainSpline))
  (bind _returnvalue (StaticMesh|GetBoundingBox _chainlink))
  (bind _returnvalue_2 (- 0.0 _chain_length))
  (Transformation|AddLocalOffset (Variables|Default|GetSM_IronChandelier) (Math|Vector|MakeVector 0.0 0.0 _returnvalue_2) false false)
  (Spline|SetLocationatSplinePoint (Variables|Default|GetChainSpline) 1 (Math|Vector|MakeVector 0.0 0.0 (+ _returnvalue_2 -17.919437)) "Local" true)
  (bind _output_get (Variables|Default|SetLinkLength (+ 0.0 (.z (+ (Math|Vector|VectorGetAbs (.min _returnvalue)) (Math|Vector|VectorGetAbs (.max _returnvalue)))))))
  (for _index (range 0 (Math|Float|Truncate (/ (Spline|GetSplineLength (Variables|Default|GetChainSpline)) _output_get)))
    (bind _returnvalue_3 (AddComponent|AddSplineMeshComponent false))
    (SplineMesh|SetForwardAxis _returnvalue_3 "Z" true)
    (Components|StaticMesh|SetStaticMesh _returnvalue_3 (Variables|Default|GetChainLink))
    (SplineMesh|SetStartandEnd _returnvalue_3 (Spline|GetLocationatDistanceAlongSpline _chainspline (* _index (Variables|Default|GetLinkLength)) "Local") (Math|Vector|ClampVectorSize (Spline|GetTangentatDistanceAlongSpline _chainspline (* _index (Variables|Default|GetLinkLength)) "Local") 0.0 (Variables|Default|GetLinkLength)) (Spline|GetLocationatDistanceAlongSpline _chainspline (* (+ _index 1) (Variables|Default|GetLinkLength)) "Local") (Math|Vector|ClampVectorSize (Spline|GetTangentatDistanceAlongSpline _chainspline (* (+ _index 1) (Variables|Default|GetLinkLength)) "Local") 0.0 (Variables|Default|GetLinkLength)) true :!class /Script/Engine.SplineMeshComponent)))