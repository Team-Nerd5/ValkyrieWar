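; Construction-script prop for the castle town that stretches a single chain mesh between the two points of a spline.
; When ActorSelected is set, both points take the world locations of ActorBase and ActorTarget, written as local-space coordinates.
; The mesh rotates toward the second point, and spline length selects one of four chain sizes, scaled along X to fit.
; LooseChain selects loose variants for all but the smallest size.
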(event EventBeginPlay)

(event Collision|EventActorBeginOverlap
  (params (OtherActor :type Actor%20Object%20Reference)))

(event EventTick
  (params (DeltaSeconds :type Float%20%28single-precision%29)))

(fn ConstructionScript
  (bind _chainmesh (Variables|Default|GetChainMesh))
  (bind _chainmesh_2 (Variables|Default|GetChainMesh))
  (bind _spline (Variables|Default|GetSpline))
  (if (Variables|Default|GetActor%20Selected)
    (Spline|SetLocationatSplinePoint (Variables|Default|GetSpline) 1 (Transformation|GetActorLocation (Variables|Default|GetActor%20Target)) "Local" true)
    (Spline|SetLocationatSplinePoint (Variables|Default|GetSpline) 0 (Transformation|GetActorLocation (Variables|Default|GetActor%20Base)) "Local" true))
  (Transformation|SetRelativeRotation (Variables|Default|GetChainMesh) (Math|Rotator|FindLookatRotation (Spline|GetLocationatSplinePoint _spline 0 "Local") (Spline|GetLocationatSplinePoint _spline 1 "Local")) false false)
  (bind _output_get (Variables|Default|SetLength (Spline|GetSplineLength (Variables|Default|GetSpline))))
  (if (<= _output_get 1.1e+02)
    (Components|StaticMesh|SetStaticMesh (Variables|Default|GetChainMesh) "/Game/ExternalContents/Environments/Castle/CastleTown/Static_Mesh/Props/Chains/SM_Chain_Small.SM_Chain_Small")
    (Transformation|SetRelativeScale3D (Variables|Default|GetChainMesh) (Math|Vector|MakeVector (/ (Variables|Default|GetLength) 81.0) 1.0 1.0))
    (elif (<= (Variables|Default|GetLength) 2e+02)
      (if (Variables|Default|GetLooseChain)
        (Components|StaticMesh|SetStaticMesh _chainmesh_2 "/Game/ExternalContents/Environments/Castle/CastleTown/Static_Mesh/Props/Chains/SM_Chain_Med_Loose.SM_Chain_Med_Loose")
        (else
          (Components|StaticMesh|SetStaticMesh _chainmesh_2 "/Game/ExternalContents/Environments/Castle/CastleTown/Static_Mesh/Props/Chains/SM_Chain_Med.SM_Chain_Med")))
      (Transformation|SetRelativeScale3D (Variables|Default|GetChainMesh) (Math|Vector|MakeVector (/ (Variables|Default|GetLength) 144.0) 1.0 1.0))
      (elif (<= (Variables|Default|GetLength) 3e+02)
        (if (Variables|Default|GetLooseChain)
          (Components|StaticMesh|SetStaticMesh _chainmesh "/Game/ExternalContents/Environments/Castle/CastleTown/Static_Mesh/Props/Chains/SM_Chain_Long_Loose.SM_Chain_Long_Loose")
          (else
            (Components|StaticMesh|SetStaticMesh _chainmesh "/Game/ExternalContents/Environments/Castle/CastleTown/Static_Mesh/Props/Chains/SM_Chain_Long.SM_Chain_Long")))
        (Transformation|SetRelativeScale3D (Variables|Default|GetChainMesh) (Math|Vector|MakeVector (/ (Variables|Default|GetLength) 257.0) 1.0 1.0))
        (else
          (if (Variables|Default|GetLooseChain)
            (Components|StaticMesh|SetStaticMesh (Variables|Default|GetChainMesh) "/Game/ExternalContents/Environments/Castle/CastleTown/Static_Mesh/Props/Chains/SM_Chain_XtraLong_Loose.SM_Chain_XtraLong_Loose")
            (else
              (Components|StaticMesh|SetStaticMesh (Variables|Default|GetChainMesh) "/Game/ExternalContents/Environments/Castle/CastleTown/Static_Mesh/Props/Chains/SM_Chain_XtraLong.SM_Chain_XtraLong")))
          (Transformation|SetRelativeScale3D (Variables|Default|GetChainMesh) (Math|Vector|MakeVector (/ (Variables|Default|GetLength) 579.0) 1.0 1.0)))))))