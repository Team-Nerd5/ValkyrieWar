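; PC_InventoryTest is a test player controller Blueprint for exercising the inventory system and its UI.
; BeginPlay creates and opens WBP_Inventory, initializes test item data through the GameManager game instance, then has the InventorySystem add test items.
; Debug keys switch between Manual and Auto control modes with an on-screen print, and open or close the inventory.
; An unconnected leftover block fills the widget with dummy list objects.
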(event EventBeginPlay
  (Utilities|FlowControl|Sequence
    (:then_0
      (bind _returnvalue (UserInterface|CreateWidget "/Game/Test/OKM/Inventory/WBP_Inventory.WBP_Inventory_C"))
      (UserInterface|Viewport|AddtoViewport _returnvalue 0)
      (Class|TestInventoryWidget|OpenUI _returnvalue))
    (:then_1
      (bind _asgame_manager (Utilities|Casting|CastToGameManager (Game|GetGameInstance)))
      (Class|DataManager|InitTestItem (Subsystems|GetDataManager) _asgame_manager))
    (:then_2
      (Class|InventorySystem|TestAddItem (Subsystems|GetInventorySystem)))))

(event Input|KeyboardEvents|DebugKey1
  (params (Key :type Key%20Structure :default "None") (ActionValue :type Input%20Action%20Value%20Structure))
  (:Pressed
    (Development|PrintString "메뉴얼!")
    (Class|ValkyrieCharacterController|SetControlMode "Manual")))

(event Input|KeyboardEvents|DebugKey2
  (params (Key :type Key%20Structure :default "None") (ActionValue :type Input%20Action%20Value%20Structure))
  (:Pressed
    (Development|PrintString "오토!")
    (Class|ValkyrieCharacterController|SetControlMode "Auto")))

(event Input|KeyboardEvents|DebugKey3
  (params (Key :type Key%20Structure :default "None") (ActionValue :type Input%20Action%20Value%20Structure))
  (:Pressed
    (Class|TestInventoryWidget|OpenUI (stale EventBeginPlay _returnvalue))))

(event Input|KeyboardEvents|DebugKey4
  (params (Key :type Key%20Structure :default "None") (ActionValue :type Input%20Action%20Value%20Structure))
  (:Pressed
    (Class|TestInventoryWidget|CloseUI (stale EventBeginPlay _returnvalue))))

(event Input|KeyboardEvents|DebugKey5
  (params (Key :type Key%20Structure :default "None") (ActionValue :type Input%20Action%20Value%20Structure)))

(fn ConstructionScript)