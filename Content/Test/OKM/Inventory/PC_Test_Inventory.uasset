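; Test player controller for exercising the inventory UI and inventory system.
; On BeginPlay it creates a WBP_Inventory widget, adds it to the viewport and starts it closed.
; Debug keys then add a test item through the InventorySystem, open or close the widget, and switch it between inventory and character info popup types.
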(event EventBeginPlay
  (Utilities|FlowControl|Sequence
    (:then_0
      (bind _returnvalue (UserInterface|CreateWidget "/Game/Widget/Popup/Inventory/WBP_Inventory.WBP_Inventory_C"))
      (UserInterface|Viewport|AddtoViewport _returnvalue 0)
      (Class|InventoryWidget|CloseUI _returnvalue))))

(event Input|KeyboardEvents|DebugKey1
  (params (Key :type Key%20Structure :default "None") (ActionValue :type Input%20Action%20Value%20Structure))
  (:Pressed
    (Class|InventoryWidget|CloseUI (stale EventBeginPlay _returnvalue))))

(event Input|KeyboardEvents|DebugKey2
  (params (Key :type Key%20Structure :default "None") (ActionValue :type Input%20Action%20Value%20Structure))
  (:Pressed
    (Class|InventoryWidget|OpenUI (stale EventBeginPlay _returnvalue))))

(event Input|KeyboardEvents|DebugKey3
  (params (Key :type Key%20Structure :default "None") (ActionValue :type Input%20Action%20Value%20Structure))
  (:Pressed
    (Class|InventoryWidget|UpdateInventoryType (stale EventBeginPlay _returnvalue) "PopupInventory")))

(event Input|KeyboardEvents|DebugKey4
  (params (Key :type Key%20Structure :default "None") (ActionValue :type Input%20Action%20Value%20Structure))
  (:Pressed
    (Class|InventoryWidget|UpdateInventoryType (stale EventBeginPlay _returnvalue) "PopupCharacterInfo")))

(event Input|KeyboardEvents|DebugKey0
  (params (Key :type Key%20Structure :default "None") (ActionValue :type Input%20Action%20Value%20Structure))
  (:Pressed
    (Class|InventorySystem|TestAddItem (Subsystems|GetInventorySystem))))

(fn ConstructionScript)