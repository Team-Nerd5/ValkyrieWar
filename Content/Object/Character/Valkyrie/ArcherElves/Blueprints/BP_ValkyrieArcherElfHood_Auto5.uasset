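; Valkyrie hooded archer elf character (Auto5 variant) whose only live graph logic is a debug bow attack trigger.
; Pressing debug key T tries to activate GA_BowAttack_BP through its Ability System Component and prints the result.
; Leftover nodes for creating a WBP_MoveUI joystick widget and feeding its axes into movement input are disconnected and never run.
; BeginPlay, overlap, Tick and the construction script are empty.
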(event EventBeginPlay)

(event Collision|EventActorBeginOverlap
  (params (OtherActor :type Actor%20Object%20Reference)))

(event EventTick
  (params (DeltaSeconds :type Float%20%28single-precision%29)))

(event Input|KeyboardEvents|DebugKeyT
  (params (Key :type Key%20Structure :default "None") (ActionValue :type Input%20Action%20Value%20Structure))
  (:Pressed
    (Development|PrintString "Hello")
    (bind _returnvalue (Abilities|TryActivateAbilitybyClass (Ability|GetAbilitySystemComponent 0) "/Game/Object/Character/Weapon/Range/GA_BowAttack_BP.GA_BowAttack_BP_C" true))
    (Development|PrintString (Utilities|String|ToString(Boolean) _returnvalue))))

(fn ConstructionScript)